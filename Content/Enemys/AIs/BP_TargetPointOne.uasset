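; BP_TargetPointOne is a target point in the enemy AI folder that jumps between fixed world locations.
; From BeginPlay, it moves its root component through four hardcoded positions without sweeping, waiting three seconds at each, then loops back to the first indefinitely.
; The loop is a chain of Delay nodes wired back to its start, with debug prints of the current location after the first three waits.
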(event `self.ReceiveBeginPlay`
  (set `self.Root Component` (`self.RootComponent`))
  (`SceneComponent.K2_SetWorldLocation` (`self.Root Component`) (-605.0 -1845.0 20.0) false false :!label _label)
  (`KismetSystemLibrary.Delay` 3.0)
  (`KismetSystemLibrary.PrintString` (`KismetStringLibrary.Conv_VectorToString` (`SceneComponent.K2_GetComponentLocation` (`self.Root Component`))))
  (`SceneComponent.K2_SetWorldLocation` (`self.Root Component`) (1785.0 1845.0 20.0) false false)
  (`KismetSystemLibrary.Delay` 3.0)
  (`KismetSystemLibrary.PrintString` (`KismetStringLibrary.Conv_VectorToString` (`SceneComponent.K2_GetComponentLocation` (`self.Root Component`))))
  (`SceneComponent.K2_SetWorldLocation` (`self.Root Component`) (1785.0 -735.0 20.0) false false)
  (`KismetSystemLibrary.Delay` 3.0)
  (`KismetSystemLibrary.PrintString` (`KismetStringLibrary.Conv_VectorToString` (`SceneComponent.K2_GetComponentLocation` (`self.Root Component`))))
  (`SceneComponent.K2_SetWorldLocation` (`self.Root Component`) (15.0 2456.0 20.0) false false)
  (`KismetSystemLibrary.Delay` 3.0)
  (goto _label))

(fn `UserConstructionScript`)